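; 3D minimap actor that shows a miniature of the static world around the player, with markers for player and nearby artifacts.
; On BeginPlay it clones WorldStatic meshes from the pawn's Maparea as collision-free, forced-LOD components shrunk by ScaleDivider.
; Seven pooled cubes mark ArtifactArea collectables, leftovers are hidden, and Refresh re-places them.
; Tick moves the player cylinder; the older whole-world scan is disconnected.
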(event `self.ReceiveBeginPlay`
  ;[1 1 1] Event BeginPlay | Main operation
  (`self.PrepBeOp`)
  (`self.CreateWorldMap`)
  (`self.AddPlayer`)
  (`self.DisplayArtifact`)
  (`self.Spawn Collectables`)
  (`self.Hide unwanted Cube`))

(event `PrepBeOp`
  (bind _cubearray (`self.CubeArray`))
  ;[1 1 1] PrepBeOp | Preperation Before Operation
  (`KismetArrayLibrary.Array_Clear` (`self.OverlappingActors`))
  (`KismetArrayLibrary.Array_Clear` (`self.Collectables`))
  (if (== (`KismetArrayLibrary.Array_Length` (`self.CubeArray`)) 7)
    (for _array_element (`self.CubeArray`)
      (`SceneComponent.K2_SetRelativeLocation` _array_element (0.0 0.0 0.0) false false)
      (`self.GetAllStaticMeshInArea` :!label _label))
    (else
      (`KismetArrayLibrary.Array_Add` _cubearray (`self.Cube1`))
      (`KismetArrayLibrary.Array_Add` _cubearray (`self.Cube2`))
      (`KismetArrayLibrary.Array_Add` _cubearray (`self.Cube3`))
      (`KismetArrayLibrary.Array_Add` _cubearray (`self.Cube4`))
      (`KismetArrayLibrary.Array_Add` _cubearray (`self.Cube5`))
      (`KismetArrayLibrary.Array_Add` _cubearray (`self.Cube6`))
      (`KismetArrayLibrary.Array_Add` _cubearray (`self.Cube7`))
      (goto _label))))

(event `GetAllStaticMeshInArea`
  ;[1 1 1] Get all static mesh around player
  (bind _asmotion_controller_pawn (cast `/Game/VirtualRealityBP/Blueprints/MotionControllerPawn` (`GameplayStatics.GetPlayerCharacter` 0)))
  (bind _output_get (set `self.PlayerRef` _asmotion_controller_pawn))
  (for _array_element (`/Game/VirtualRealityBP/Blueprints/MotionControllerPawn.Maparea` _output_get)
    (bind _asstatic_mesh_actor (cast `StaticMeshActor` _array_element))
    (if (`|EnumEquality` (`PrimitiveComponent.GetCollisionObjectType` (`StaticMeshActor.StaticMeshComponent` _asstatic_mesh_actor)) "ECC_WorldStatic")
      (`KismetArrayLibrary.Array_Add` (`self.WorldMeshActors`) _asstatic_mesh_actor))))

(event `DisplayArtifact`
  ;[1 1 1] Display artifact near player
  (for _array_element (`/Game/VirtualRealityBP/Blueprints/MotionControllerPawn.ArtifactArea` (`self.PlayerRef`))
    (`KismetArrayLibrary.Array_Add` (`self.Collectables`) _array_element)))

(event `Hide unwanted Cube`
  ;[1 1 1] Hide unwanted cube
  (for _array_element (`self.CubeArray`)
    (if (`KismetMathLibrary.EqualExactly_VectorVector` (`SceneComponent.RelativeLocation` _array_element))
      (`SceneComponent.SetHiddenInGame` _array_element true false))))

(event `Refresh`
  ;[1 1 1] Refresh Collectable location and availability
  (`self.Spawn Collectables`)
  (set `self.RefreshArtifactLocal` false))

(event `GetAllStaticActors`
  ;[1 1 1] Get all static mesh actor in world
  (bind _outactors (`GameplayStatics.GetAllActorsOfClass` "/Script/Engine.StaticMeshActor"))
  (for _array_element _outactors
    (if (`|EnumEquality` (`PrimitiveComponent.GetCollisionObjectType` (`StaticMeshActor.StaticMeshComponent` _array_element)) "ECC_WorldStatic")
      (`KismetArrayLibrary.Array_Add` (`self.WorldMeshActors`) _array_element))))

(event `CreateWorldMap`
  (bind _scaledivider (`self.ScaleDivider`))
  ;[1 1 1] Create world with static mesh data
  (for _array_element (`self.WorldMeshActors`)
    (switch `string` (`KismetSystemLibrary.GetObjectName` _array_element)
      (:`Default`
        (bind _staticmeshcomponent (`StaticMeshActor.StaticMeshComponent` _array_element))
        (bind (_returnvalue_location _returnvalue_rotation _returnvalue_scale) (`KismetMathLibrary.BreakTransform` (`SceneComponent.K2_GetComponentToWorld` _staticmeshcomponent)))
        (bind _returnvalue (`AddComponent|NODE_AddStaticMeshComponent-0` :`RelativeTransform` (`KismetMathLibrary.MakeTransform` (`KismetMathLibrary.TransformLocation` (`self.GetTransform` self) (/ _returnvalue_location _scaledivider)) _returnvalue_rotation (/ _returnvalue_scale _scaledivider))))
        (`PrimitiveComponent.SetCollisionObjectType` _returnvalue "ECC_WorldDynamic")
        (`PrimitiveComponent.SetCollisionEnabled` _returnvalue "NoCollision")
        (`StaticMeshComponent.SetStaticMesh` _returnvalue (`StaticMeshComponent.StaticMesh` _staticmeshcomponent))
        (`StaticMeshComponent.SetForcedLodModel` _returnvalue 2)))))

(event `AddPlayer`
  (bind _player_cylinder (`self.Player Cylinder`))
  (bind (_returnvalue_location _returnvalue_rotation _returnvalue_scale) (`KismetMathLibrary.BreakTransform` (`SceneComponent.K2_GetComponentToWorld` (`Actor.RootComponent` (`self.PlayerRef`)))))
  ;[1 1 1] Add player to world
  (`SceneComponent.K2_SetRelativeLocation` _player_cylinder (`KismetMathLibrary.TransformLocation` (`self.GetTransform` self) (/ _returnvalue_location (`self.ScaleDivider`))) false false)
  (`SceneComponent.K2_SetRelativeRotation` _player_cylinder _returnvalue_rotation false false)
  (`SceneComponent.SetRelativeScale3D` _player_cylinder (/ _returnvalue_scale 100.0))
  (`PrimitiveComponent.SetCollisionEnabled` _player_cylinder "NoCollision"))

(event `Add Collectables`
  ;[1 1 1] Add all artifact to world
  (bind _outactors (`GameplayStatics.GetAllActorsOfClass` "/Game/Assets/Clayton/Collectables/Collectables.Collectables_C"))
  (for _array_element _outactors
    (`KismetArrayLibrary.Array_Add` (`self.Collectables`) _array_element)))

(event `Spawn Collectables`
  ;[1 1 1] Spawn Artifact
  (for (_array_element _array_index) (`self.Collectables`)
    (bind _output (`|GetArrayItem` (`self.CubeArray`) _array_index))
    (`/Engine/EditorBlueprintResources/StandardMacros.IsValid` _output
      (:`Is Valid`
        (bind (_returnvalue_location _returnvalue_rotation _returnvalue_scale) (`KismetMathLibrary.BreakTransform` (`SceneComponent.K2_GetComponentToWorld` (`Actor.RootComponent` (`self.GetParentActor` _array_element)))))
        (`SceneComponent.K2_SetRelativeLocation` _output (/ _returnvalue_location (`self.ScaleDivider`)) false false)
        (`SceneComponent.K2_SetRelativeRotation` _output _returnvalue_rotation false false)
        (`SceneComponent.SetRelativeScale3D` _output (/ _returnvalue_scale 100.0))
        (`PrimitiveComponent.SetCollisionEnabled` _output "NoCollision"))
      (:`Is Not Valid`
        (`SceneComponent.SetVisibility` _output false false)))))

(event `self.ReceiveTick`
  (params (DeltaSeconds :type "Float (single-precision)"))
  (bind _returnvalue_location (`KismetMathLibrary.BreakTransform` (`SceneComponent.K2_GetComponentToWorld` (`Actor.RootComponent` (`self.PlayerRef`)))))
  ;[1 1 1] Event Tick | Update player pos
  (`SceneComponent.K2_SetRelativeLocation` (`self.Player Cylinder`) (/ _returnvalue_location (`self.ScaleDivider`)) false false))

(fn `UserConstructionScript`)