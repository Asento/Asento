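; BP_3DMap builds a scaled-down 3D miniature of the level, showing the player and collectables.
; On BeginPlay it copies WorldStatic static mesh actors, except WaterPlane, as collision-free mesh components with positions and scales shrunk by ScaleDivider.
; Collectables become cube markers placed from their parent actors' transforms.
; A Cube component marks the player, and Tick updates its relative location from the scaled player position.
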(event `self.ReceiveBeginPlay`
  (`self.GetAllStaticActors`)
  (`self.CreateWorldMap`)
  (`self.AddPlayer`)
  (`self.Add Collectables`)
  (`self.Spawn Collectables`))

(event `GetAllStaticActors`
  (bind _outactors (`GameplayStatics.GetAllActorsOfClass` "/Script/Engine.StaticMeshActor"))
  (for _array_element _outactors
    (if (`|EnumEquality` (`PrimitiveComponent.GetCollisionObjectType` (`StaticMeshActor.StaticMeshComponent` _array_element)) "ECC_WorldStatic")
      (`KismetArrayLibrary.Array_Add` (`self.WorldMeshActors`) _array_element))))

(event `CreateWorldMap`
  (bind _scaledivider (`self.ScaleDivider`))
  (for _array_element (`self.WorldMeshActors`)
    (if (`KismetStringLibrary.NotEqual_StrStr` (`KismetSystemLibrary.GetDisplayName` _array_element) "WaterPlane")
      (bind _staticmeshcomponent (`StaticMeshActor.StaticMeshComponent` _array_element))
      (bind (_returnvalue_location _returnvalue_rotation _returnvalue_scale) (`KismetMathLibrary.BreakTransform` (`SceneComponent.K2_GetComponentToWorld` _staticmeshcomponent)))
      (bind _returnvalue (`AddComponent|NODE_AddStaticMeshComponent-0` :`RelativeTransform` (`KismetMathLibrary.MakeTransform` (`KismetMathLibrary.TransformLocation` (`self.GetTransform` self) (/ _returnvalue_location _scaledivider)) _returnvalue_rotation (/ _returnvalue_scale _scaledivider))))
      (`PrimitiveComponent.SetCollisionObjectType` _returnvalue "ECC_WorldDynamic")
      (`PrimitiveComponent.SetCollisionEnabled` _returnvalue "NoCollision")
      (`StaticMeshComponent.SetStaticMesh` _returnvalue (`StaticMeshComponent.StaticMesh` _staticmeshcomponent)))))

(event `AddPlayer`
  (bind _cube (`self.Cube`))
  (bind _asmotion_controller_pawn (cast `/Game/VirtualRealityBP/Blueprints/MotionControllerPawn` (`GameplayStatics.GetPlayerCharacter` 0)))
  (bind (_returnvalue_location _returnvalue_rotation _returnvalue_scale) (`KismetMathLibrary.BreakTransform` (`SceneComponent.K2_GetComponentToWorld` (`Actor.RootComponent` _asmotion_controller_pawn))))
  (`SceneComponent.K2_SetRelativeLocation` _cube (`KismetMathLibrary.TransformLocation` (`self.GetTransform` self) (/ _returnvalue_location (`self.ScaleDivider`))) false false)
  (`SceneComponent.K2_SetRelativeRotation` _cube _returnvalue_rotation false false)
  (`SceneComponent.SetRelativeScale3D` _cube (/ _returnvalue_scale 100.0))
  (`PrimitiveComponent.SetCollisionEnabled` _cube "NoCollision"))

(event `Add Collectables`
  (bind _outactors (`GameplayStatics.GetAllActorsOfClass` "/Game/Assets/Clayton/Collectables.Collectables_C"))
  (for _array_element _outactors
    (`KismetArrayLibrary.Array_Add` (`self.Collectables`) _array_element)))

(event `Spawn Collectables`
  (for _array_element (`self.Collectables`)
    (bind (_returnvalue_location _returnvalue_rotation _returnvalue_scale) (`KismetMathLibrary.BreakTransform` (`SceneComponent.K2_GetComponentToWorld` (`Actor.RootComponent` (`self.GetParentActor` _array_element)))))
    (bind _returnvalue (`AddComponent|NODE_AddStaticMeshComponent-6` :`RelativeTransform` (`KismetMathLibrary.MakeTransform` (`KismetMathLibrary.TransformLocation` (`self.GetTransform` self) (/ _returnvalue_location (`self.ScaleDivider`))) _returnvalue_rotation (/ _returnvalue_scale 20.0))))
    (`PrimitiveComponent.SetCollisionObjectType` _returnvalue "ECC_WorldDynamic")
    (`PrimitiveComponent.SetCollisionEnabled` _returnvalue "NoCollision")
    (`StaticMeshComponent.SetStaticMesh` _returnvalue "/Game/Geometry/Meshes/1M_Cube.1M_Cube")))

(event `self.ReceiveTick`
  (params (DeltaSeconds :type "Float (single-precision)"))
  (bind _returnvalue_location (`KismetMathLibrary.BreakTransform` (`SceneComponent.K2_GetComponentToWorld` (`Actor.RootComponent` (`GameplayStatics.GetPlayerCharacter` 0)))))
  (`SceneComponent.K2_SetRelativeLocation` (`self.Cube`) (/ _returnvalue_location (`self.ScaleDivider`)) false false))

(fn `UserConstructionScript`)